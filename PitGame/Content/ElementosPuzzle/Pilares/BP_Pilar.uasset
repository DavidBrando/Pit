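; BP_Pilar is a puzzle pillar that captures CuboPadre cubes entering its collider.
; On overlap with a physics-simulating cube, its own Physics Handle grabs the cube's mesh using the Scene component's world location.
; It then messages the player character to reset their physics handle and registers itself as the cube's pillar.
; The releaseObject event lets go of the held cube.
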(event `self.CubeCollider.OnComponentBeginOverlap`
  (params (OverlappedComponent :type "PrimitiveComponent Object Reference") (OtherActor :type "Actor Object Reference") (OtherComp :type "PrimitiveComponent Object Reference") (OtherBodyIndex :type Integer) (bFromSweep :type Boolean) (SweepResult :type "HitResult Structure (by ref)"))
  (`/Engine/EditorBlueprintResources/StandardMacros.IsValid` OtherActor
    (:`Is Valid`
      (bind _ascubo_padre (cast `/Game/ElementosPuzzle/Cubos/CuboPadre` OtherActor))
      (bind _staticmesh (`/Game/ElementosPuzzle/Cubos/CuboPadre.StaticMesh` _ascubo_padre))
      (if (`SceneComponent.IsSimulatingPhysics` _staticmesh "None")
        (`PhysicsHandleComponent.GrabComponentAtLocationWithRotation` :`self` (`self.PhysicsHandle`) :`Component` _staticmesh :`Location` (`SceneComponent.K2_GetComponentLocation` (`self.Scene`)))
        (message `/Game/ElementosPuzzle/BPI_PuzzleElements_PlayerComunication.ResetPlayerPhysicsHandle` (`GameplayStatics.GetPlayerCharacter` 0))
        (`/Game/ElementosPuzzle/Cubos/CuboPadre.setPillar` _ascubo_padre self)))))

(event `releaseObject`
  (`PhysicsHandleComponent.ReleaseComponent` (`self.PhysicsHandle`)))

(fn `UserConstructionScript`)