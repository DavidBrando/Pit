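; Pressure plate puzzle element that plays a level sequence when a CuboPadre-derived cube or an actor of the player character's class steps on it.
; The construction script creates the sequence player, and the collider's begin overlap plays it once, guarded by the HaveAnyObject flag.
; Any end overlap clears the flag and reverses the sequence, without checking which actor left or whether others remain.
; Both overlap events print debug strings.
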(event `self.colliderDetection.OnComponentBeginOverlap`
  (params (OverlappedComponent :type "PrimitiveComponent Object Reference") (OtherActor :type "Actor Object Reference") (OtherComp :type "PrimitiveComponent Object Reference") (OtherBodyIndex :type Integer) (bFromSweep :type Boolean) (SweepResult :type "HitResult Structure (by ref)"))
  (bind _returnvalue (`GameplayStatics.GetObjectClass` OtherActor))
  (`/Engine/EditorBlueprintResources/StandardMacros.IsValid` OtherActor
    (:`Is Valid`
      (if (or (`KismetMathLibrary.ClassIsChildOf` _returnvalue "/Game/ElementosPuzzle/Cubos/CuboPadre.CuboPadre_C") (== _returnvalue (`GameplayStatics.GetObjectClass` (`GameplayStatics.GetPlayerCharacter` 0))))
        (`KismetSystemLibrary.PrintString` (`KismetSystemLibrary.GetClassDisplayName` _returnvalue))
        (if (not (`self.haveAnyObject`))
          (set `self.haveAnyObject` true)
          (`MovieSceneSequencePlayer.Play` (`LevelSequenceActor.SequencePlayer` (`self.MySequence`))))))))

(event `self.colliderDetection.OnComponentEndOverlap`
  (params (OverlappedComponent :type "PrimitiveComponent Object Reference") (OtherActor :type "Actor Object Reference") (OtherComp :type "PrimitiveComponent Object Reference") (OtherBodyIndex :type Integer))
  (`KismetSystemLibrary.PrintString` "me fui")
  (set `self.haveAnyObject` false)
  (`MovieSceneSequencePlayer.PlayReverse` (`LevelSequenceActor.SequencePlayer` (`self.MySequence`))))

(fn `UserConstructionScript`
  (bind (_outactor _returnvalue) (`LevelSequencePlayer.CreateLevelSequencePlayer` "/Game/ElementosPuzzle/Puertas/MatineeActorLevelSequence.MatineeActorLevelSequence"))
  (set `self.ActorReference` _returnvalue)
  (set `self.MySequence` _outactor))